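; BP_TireEnemy is a rolling tire enemy that patrols random target points and charges the player when nearby.
; Tick sets movement velocity by state, turns it toward travel and spins the tire.
; Proximity spawns a BP_Target marker at the player, locking a straight, faster charge until a timer restores patrol.
; Hitting a non-invincible player asks the game mode to change the player pawn, with a cooldown.
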(event OnComponentBeginOverlap(HitBox)
  (params (OverlappedComponent :type Primitive%20Component%20Object%20Reference) (OtherActor :type Actor%20Object%20Reference) (OtherComp :type Primitive%20Component%20Object%20Reference) (OtherBodyIndex :type Integer) (bFromSweep :type Boolean) (SweepResult :type Hit%20Result%20Structure%20%28by%20ref%29))
  (if (== (Pawn|GetControlledPawn (Game|GetPlayerController 0)) OtherActor)
    (if (not (Variables|/Game/Characters/BP_RespawnInvincibilityTimer.BP_RespawnInvincibilityTimer_C|GetisInvincible (Actor|GetComponentbyClass OtherActor "/Game/Characters/BP_RespawnInvincibilityTimer.BP_RespawnInvincibilityTimer_C")))
      (Utilities|FlowControl|DoOnce false :!label _label
        (:Completed
          (Utilities|FlowControl|Sequence
            (:then_0
              (bind _asbp_third_person_game_mode (Utilities|Casting|CastToBP_ThirdPersonGameMode (Game|GetGameMode)))
              (Default|ChangePlayerPawn _asbp_third_person_game_mode "NewEnumerator1"))
            (:then_1
              (Utilities|FlowControl|Delay 3.0)
              (goto _label Reset))))))))

(event Custom|Clear%20Timer
  (Actor|DestroyActor (Variables|Default|GetPlayer%20Target%20Point))
  (Variables|Default|SetTire%20Rotation%20Rate "-10.000000,0.000000,0.000000")
  (Variables|Default|SetEnemy%20State "NewEnumerator0")
  (Utilities|FlowControl|DoOnce false) ; enters at Reset
)

(event EventBeginPlay
  (CallFunction|FindTarget)
  (Variables|Default|SetTire%20Rotation%20Rate "-10.000000,0.000000,0.000000"))

(event EventTick
  (params (DeltaSeconds :type Float%20%28single-precision%29))
  (bind _returnvalue (Game|GetPlayerController 0))
  (bind _returnvalue_2 (Transformation|GetActorLocation))
  (bind _returnvalue_3 (Pawn|GetControlledPawn _returnvalue))
  (Utilities|FlowControl|Sequence
    (:then_0
      (switch Utilities|FlowControl|Switch|SwitchonETireEnemyStates (Variables|Default|GetEnemy%20State)
        (:NewEnumerator0
          (if (Utilities|Operators|NotEqual(!=) :A (Variables|Default|GetTarget%20Location))
            (bind _output_get (Variables|Default|SetDir (Math|Vector|Normalize (- (Variables|Default|GetTarget%20Location) (Transformation|GetActorLocation)))))
            (Variables|/Script/Engine.MovementComponent|SetVelocity (Variables|Character|GetCharacterMovement) (* _output_get 1e+03))
            (if (Variables|Default|GetIsAtPoint)
              (Variables|Default|SetTire%20Rotation%20Rate "0, 0, 0")
              (Utilities|FlowControl|Delay 5.0)
              (Variables|Default|SetIsAtPoint false)
              (CallFunction|FindTarget))))
        (:NewEnumerator1
          (Variables|/Script/Engine.MovementComponent|SetVelocity (Variables|Character|GetCharacterMovement) (* (Variables|Default|GetDir) 2.5e+03)))))
    (:then_1
      (bind _output_get_2 (Variables|Default|SetTarget%20Rotation (Math|Rotator|FindLookatRotation _returnvalue_2 (+ (Transformation|GetVelocity) _returnvalue_2))))
      (Transformation|SetActorRotation (Math|Interpolation|RInterpTo (Transformation|GetActorRotation) _output_get_2 DeltaSeconds 1e+01))
      (Transformation|AddLocalRotation (Variables|Default|GetTire) (Variables|Default|GetTire%20Rotation%20Rate) false false))
    (:then_2
      (if (<= (Transformation|GetDistanceTo _returnvalue_3) 1e+03)
        (Utilities|FlowControl|DoOnce false
          (:Completed
            (bind _returnvalue_4 (Game|SpawnActorfromClass "/Game/Blueprints/BP_Target.BP_Target_C" (Math|Transform|MakeTransform (Transformation|GetActorLocation _returnvalue_3) "0, 0, 0" "1.000000,1.000000,1.000000") "Undefined" "MultiplyWithRoot" 0 0))
            (bind _output_get_3 (Variables|Default|SetPlayer%20Target%20Point _returnvalue_4))
            (Development|SetHiddeninGame (Variables|/Game/Blueprints/BP_Target.BP_Target_C|GetSphere _output_get_3) false true)
            (Variables|Default|SetEnemy%20State "NewEnumerator1")
            (Variables|Default|SetDir (Math|Vector|Normalize (- (Transformation|GetActorLocation _returnvalue_4) (Transformation|GetActorLocation))))
            (Variables|Default|SetTire%20Rotation%20Rate "-20.000000,0.000000,0.000000")
            (Utilities|Time|SetTimerbyEvent (delegate Custom|Clear%20Timer) 1.5)))))))

(fn ConstructionScript)

(fn FindTarget
  (bind _targetpoints (Variables|Default|GetTargetPoints))
  (Utilities|Array|Shuffle _targetpoints)
  (Variables|Default|SetTarget%20Location (Transformation|GetActorLocation (.OutItem (Utilities|Array|Random _targetpoints)))))