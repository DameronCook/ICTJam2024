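; BP_SpaceMan is an actor that tracks the player's pawn and fires BP_LaserMan actors when the pawn comes close.
; Each Tick it smoothly interpolates its rotation from the SMSpaceBoy mesh toward the pawn and checks their distance.
; Within range, it prints a debug message, and a Delay in Tick throttles spawning to roughly once per second.
; Each spawned laser receives the forward direction and a mesh-aligned rotation.
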(event EventBeginPlay)

(event Collision|EventActorBeginOverlap
  (params (OtherActor :type Actor%20Object%20Reference)))

(event EventTick
  (params (DeltaSeconds :type Float%20%28single-precision%29))
  (Transformation|SetActorRotation (Math|Interpolation|RInterpTo (Transformation|GetActorRotation) (Math|Conversions|RotationFromXVector (Math|Vector|Normalize (- (Transformation|GetActorLocation (Pawn|GetControlledPawn (Game|GetPlayerController 0))) (Transformation|GetWorldLocation (Variables|Default|GetSM_SpaceBoy))))) DeltaSeconds 1e+01))
  (if (< (Math|Vector|Distance(Vector) (Transformation|GetActorLocation (Pawn|GetControlledPawn (Game|GetPlayerController 0))) (Transformation|GetWorldLocation (Variables|Default|GetSM_SpaceBoy))) 4e+03)
    (Development|PrintString "Close" true true "(R=0.000000,G=0.660000,B=1.000000,A=1.000000)" 5.0 "spaceman")
    (Utilities|FlowControl|Delay 1.0)
    (bind _returnvalue (Game|SpawnActorfromClass "/Game/Characters/SpaceMan/BP_LaserMan.BP_LaserMan_C" (Math|Transform|MakeTransform (+ (Transformation|GetActorLocation) (* (Transformation|GetActorForwardVector) 1e+02)) "0, 0, 0" "1.000000,1.000000,1.000000") "Undefined" "MultiplyWithRoot" 0 0))
    (bind _asbp_laser_man (Utilities|Casting|CastToBP_LaserMan _returnvalue))
    (Variables|/Game/Characters/SpaceMan/BP_LaserMan.BP_LaserMan_C|SetDir _asbp_laser_man (Transformation|GetActorForwardVector))
    (Transformation|SetWorldRotation (Variables|/Script/Engine.Actor|GetRootComponent _asbp_laser_man) (Math|Rotator|MakeRotator 9e+01 9e+01 (+ (.yaw (Math|Conversions|RotationFromXVector (Math|Vector|GetForwardVector (Variables|Default|GetSM_SpaceBoy)))) 9e+01)) false false)))

(fn ConstructionScript)