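; AI Brute enemy character that wanders the navmesh and chases the player, with debug prints throughout.
; Wandering moves to random points beyond a minimum distance, pausing on arrival or when a forward trace hits something.
; Perceiving the player within sight range while wandering can start a timer-driven chase, projecting the target onto the navmesh when heights differ.
; A repeating trace returns it to wandering when range or line of sight is lost, excepting "EnemyXRAY"-tagged blockers.
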(event OnTargetPerceptionUpdated(AIPerception)
  (params (Actor :type Actor%20Object%20Reference) (Stimulus :type AI%20Stimulus%20Structure))
  (if (== Actor (Pawn|GetControlledPawn (Game|GetPlayerController 0)))
    (bind _returnvalue (Class|AIPerceptionSystem|GetSenseClassforStimulus Stimulus))
    (if (== _returnvalue "/Script/AIModule.AISense_Hearing") ; Is heard?
      _
      (else
        _))
    (if (CallFunction|IsWithinSightRange)
      (switch Utilities|FlowControl|Switch|SwitchonE_AIState (Variables|Default|GetaiState)
        (:NewEnumerator0
          (switch Utilities|FlowControl|Switch|SwitchonE_AIActionType (Variables|Default|GetactionType)
            (:NewEnumerator0
              (if (Utilities|Enum|NotEqual(Enum) (Variables|Default|GetaiState) "NewEnumerator3")
                (CallFunction|BeginChase))))))
      (else
        (Development|PrintString "not within my sight")))))

(event Custom|BeginMove
  (params (moveType :type E_AIMoveType%20Enum :default "NewEnumerator0"))
  (CallFunction|StopChasing)
  (CallFunction|StopWanderTimer)
  (switch Utilities|FlowControl|Switch|SwitchonE_AIMoveType moveType
    (:NewEnumerator0
      (CallFunction|BeginWander))))

(event EventTick
  (params (DeltaSeconds :type Float%20%28single-precision%29))
  (Development|PrintString (Utilities|String|EnumtoString (Variables|Default|GetaiState)) true true "(R=1.000000,G=0.771296,B=0.000000,A=1.000000)" 2.0 "aistate"))

(event EventBeginPlay
  (Variables|Wander|SetwanderOrigin (Transformation|GetActorLocation))
  (Utilities|FlowControl|Delay 0.2)
  (CallFunction|BeginMove (Variables|Default|GetmoveType)))

(fn ConstructionScript)

(fn MinimumDistanceCheck
  (params (Destination :type Vector))
  (return (>= (Math|Vector|VectorLength (- (Transformation|GetActorLocation) Destination)) (Variables|Wander|GetwanderMinimumDistance))))

(fn DistancefromPlayer
  (params (is2D :type Boolean))
  (bind _returnvalue (Transformation|GetActorLocation))
  (bind _returnvalue_2 (Game|GetPlayerController 0))
  (bind _returnvalue_3 (Pawn|GetControlledPawn _returnvalue_2))
  (bind _returnvalue_4 (Transformation|GetActorLocation _returnvalue_3))
  (if is2D
    (return (Math|Vector|Distance2D(Vector) _returnvalue _returnvalue_4))
    (else
      (return (Math|Vector|Distance(Vector) _returnvalue _returnvalue_4)))))

(fn IsWithinSightRange
  (return (<= (CallFunction|DistancefromPlayer false) (Variables|Default|GetmaxSightRange))))

(fn StopChaseTimer)

(event Custom|WanderWalkingTimer
  (bind _returnvalue (Transformation|GetActorLocation))
  (bind _wanderwaittimevariance (Variables|Wander|GetwanderWaitTimeVariance))
  (bind _charactermovement (Variables|Character|GetCharacterMovement))
  ;[0.7219 0.7219 0.7219] Dont Wander Into Walls
  (bind _returnvalue_2 (Collision|LineTraceByChannel _returnvalue (+ _returnvalue (* (Transformation|GetActorForwardVector) (Variables|Default|GetWanderWallCheckLength))) "TraceTypeQuery1" false 0 "None"))
  (if _returnvalue_2 ; If true, stop wandering.
    (Pawn|Components|CharacterMovement|DisableMovement _charactermovement)
    (Pawn|Components|CharacterMovement|SetMovementMode _charactermovement "MOVE_NavWalking" 0)
    (Utilities|Time|ClearandInvalidateTimerbyHandle (stale _returnvalue_4) :!label _label)
    (Utilities|FlowControl|RetriggerableDelay (Math|Float|Clamp(Float) (+ (Variables|Wander|GetwanderWaitTime) (Math|Random|RandomFloatinRange (* _wanderwaittimevariance -1.0) _wanderwaittimevariance)) 0.0 99.0) :!label _label_2)
    (if (Utilities|Enum|Equal(Enum) (Variables|Default|GetaiState) "NewEnumerator0")
      (if (Variables|Default|GetwanderAroundPoint)
        (Utilities|FlowControl|Sequence
          (:then_0
            (Utilities|FlowControl|DoOnce false
              (:Completed
                (Variables|Default|SetWanderOrigin (Transformation|GetWorldLocation (Variables|Default|GetwanderPoint))))))
          (:then_1
            (bind _returnvalue_3 (Actor|GetActorOfClass "/Script/NavigationSystem.RecastNavMesh" :!label _label_3))
            (bind _randomlocation (Class|NavigationSystemV1|GetRandomLocationinNavigableRadius (Variables|Default|GetWanderOrigin) (Variables|Wander|GetwanderMaxDistance) _returnvalue_3 0 :!label _label_4))
            (if (CallFunction|MinimumDistanceCheck _randomlocation)
              (bind _returnvalue_4 (Utilities|Time|SetTimerbyEvent (delegate Custom|WanderWalkingTimer) 0.3 true))
              (AI|AIMoveTo self _randomlocation 0 5.0 false
                (:then
                  (Development|PrintString "tried to wander"))
                (:OnSuccess
                  (goto _label))
                (:OnFail
                  (Development|PrintString "WANDER FAILED")
                  (Pawn|Components|CharacterMovement|SetMovementMode (Variables|Character|GetCharacterMovement) "MOVE_NavWalking" 0)
                  (goto _label_2)))
              (else
                (Utilities|FlowControl|DelayUntilNextTick)
                (goto _label_4)))))
        (else
          (Variables|Default|SetWanderOrigin (Transformation|GetActorLocation))
          (goto _label_3)))
      (else
        (Development|PrintString "AI STATE IS NOT WANDER")
        (CallFunction|StopWanderTimer)))))

(event Custom|StopWanderTimer
  (Utilities|Time|ClearandInvalidateTimerbyHandle (stale Custom|WanderWalkingTimer _returnvalue_4))
  (Pawn|Components|CharacterMovement|DisableMovement (Variables|Character|GetCharacterMovement)))

(event Custom|BeginWander
  (bind _wanderwaittimevariance (Variables|Wander|GetwanderWaitTimeVariance))
  (bind _charactermovement (Variables|Character|GetCharacterMovement))
  (Variables|Default|SetaiState "NewEnumerator0")
  (Pawn|Components|CharacterMovement|DisableMovement _charactermovement)
  (Pawn|Components|CharacterMovement|SetMovementMode _charactermovement "MOVE_NavWalking" 0)
  (if (Variables|Default|GetwanderAroundPoint) :!label _label
    (Utilities|FlowControl|Sequence
      (:then_0
        (Utilities|FlowControl|DoOnce false
          (:Completed
            (Variables|Default|SetWanderOrigin (Transformation|GetWorldLocation (Variables|Default|GetwanderPoint))))))
      (:then_1
        (bind _returnvalue (Actor|GetActorOfClass "/Script/NavigationSystem.RecastNavMesh" :!label _label_2))
        (bind _randomlocation (Class|NavigationSystemV1|GetRandomLocationinNavigableRadius (Variables|Default|GetWanderOrigin) (Variables|Wander|GetwanderMaxDistance) _returnvalue 0 :!label _label_3))
        (if (CallFunction|MinimumDistanceCheck _randomlocation)
          (bind _returnvalue_2 (Utilities|Time|SetTimerbyEvent (delegate Custom|WanderWalkingTimer) 0.3 true))
          (AI|AIMoveTo self _randomlocation 0 5.0 false
            (:then
              (Development|PrintString "tried to wander"))
            (:OnSuccess
              (Utilities|Time|ClearandInvalidateTimerbyHandle _returnvalue_2)
              (Utilities|FlowControl|RetriggerableDelay (Math|Float|Clamp(Float) (+ (Variables|Wander|GetwanderWaitTime) (Math|Random|RandomFloatinRange (* _wanderwaittimevariance -1.0) _wanderwaittimevariance)) 0.0 99.0) :!label _label_4)
              (if (Utilities|Enum|Equal(Enum) (Variables|Default|GetaiState) "NewEnumerator0")
                (goto _label)
                (else
                  (Development|PrintString "AI STATE IS NOT WANDER")
                  (CallFunction|StopWanderTimer))))
            (:OnFail
              (Development|PrintString "WANDER FAILED")
              (Pawn|Components|CharacterMovement|SetMovementMode (Variables|Character|GetCharacterMovement) "MOVE_NavWalking" 0)
              (goto _label_4)))
          (else
            (Utilities|FlowControl|DelayUntilNextTick)
            (goto _label_3)))))
    (else
      (Variables|Default|SetWanderOrigin (Transformation|GetActorLocation))
      (goto _label_2))))

(event Custom|ChasingTraceTimer
  (bind _returnvalue (Game|GetPlayerController 0))
  (bind _returnvalue_2 (Transformation|GetActorLocation))
  (bind _returnvalue_3 (Pawn|GetControlledPawn _returnvalue))
  ;[1 1 1] Chasing Trace Checker
  (Development|PrintString "chasing trace timer")
  (bind (_outhit _returnvalue_4) (Collision|LineTraceByChannel _returnvalue_2 (+ _returnvalue_2 (* (Math|Vector|GetUnitDirection(Vector) _returnvalue_2 (Transformation|GetActorLocation _returnvalue_3)) (Variables|Default|GetmaxSightRange))) "TraceTypeQuery2" false 0 "ForDuration"))
  (if _returnvalue_4
    (if (or (== (.HitActor (Collision|BreakHitResult _outhit)) _returnvalue_3) (== (Components|GetOwner (.HitComponent (Collision|BreakHitResult _outhit))) _returnvalue_3))
      (if (CallFunction|IsWithinSightRange) :!label _label
        (Development|PrintString "still chasing" true true "(R=0.000000,G=0.660000,B=1.000000,A=1.000000)" 1.0 "")
        (else
          (CallFunction|StopChasing :!label _label_2)
          (CallFunction|BeginMove (Variables|Default|GetmoveType))
          (Development|PrintString "EXECUTED HERER" true true "(R=0.000000,G=0.660000,B=1.000000,A=1.000000)" 8.0)))
      (elif (or (Actor|ActorHasTag (.HitActor (Collision|BreakHitResult _outhit)) "EnemyXRAY") (Actor|ActorHasTag (Components|GetOwner (.HitComponent (Collision|BreakHitResult _outhit))) "EnemyXRAY"))
        (goto _label)
        (else
          (goto _label_2))))
    (else
      (goto _label_2))))

(event Custom|Chasing
  (bind _returnvalue (Game|GetPlayerController 0))
  (bind _returnvalue_2 (Pawn|GetControlledPawn _returnvalue))
  (bind _returnvalue_3 (Transformation|GetActorLocation _returnvalue_2))
  ;[1 1 1] Chasing
  (Pawn|Components|CharacterMovement|SetMovementMode (Variables|Character|GetCharacterMovement) "MOVE_NavWalking" 0)
  (bind _returnvalue_4 (Actor|GetActorOfClass "/Script/NavigationSystem.RecastNavMesh")) ; Right now will not work if there is more than one navmesh.
  (if (< (Math|Float|Absolute(Float) (- (.z (Transformation|GetActorLocation _returnvalue_2)) (.z (Transformation|GetActorLocation self)))) 5e+01)
    (Rendering|Debug|DrawDebugSphere (.RandomLocation (AI|Navigation|GetRandomReachablePointinRadius (.ProjectedLocation (AI|Navigation|ProjectPointtoNavigation _returnvalue_3 _returnvalue_4 0 (Math|Vector|MakeVector 3e+02 3e+02 1e+03))) 5e+01 0 0)) 1e+02 12 "(R=1.000000,G=0.000000,B=0.665409,A=1.000000)" 1.0 3.0)
    (AI|AIMoveTo self _returnvalue_3 _returnvalue_2 5.0 false
      (:OnFail
        (Development|PrintString "failed to walk to me")))
    (elif (.ReturnValue (AI|Navigation|ProjectPointtoNavigation (Transformation|GetActorLocation _returnvalue_2) _returnvalue_4 0 (Math|Vector|MakeVector 3e+02 3e+02 1e+03)))
      (AI|AIMoveTo self (.ProjectedLocation (AI|Navigation|ProjectPointtoNavigation (Transformation|GetActorLocation _returnvalue_2) _returnvalue_4 0 (Math|Vector|MakeVector 3e+02 3e+02 1e+03))) 0 5.0 false)
      (else
        (Development|PrintString "jumped higher than enemy sight" false)))))

(event Custom|BeginChase
  (bind _charactermovement (Variables|Character|GetCharacterMovement))
  (Development|PrintString "CHASE ACTIVATED" true true "(R=0.000000,G=0.660000,B=1.000000,A=1.000000)" 4.0)
  (Variables|/Script/Engine.CharacterMovementComponent|SetMaxWalkSpeed (Variables|Character|GetCharacterMovement) (Variables|Chase|GetChaseSpeed))
  (Variables|Default|SetaiState "NewEnumerator3")
  (CallFunction|StopWanderTimer)
  (Pawn|Components|CharacterMovement|DisableMovement _charactermovement)
  (Pawn|Components|CharacterMovement|SetMovementMode _charactermovement "MOVE_NavWalking" 0)
  (bind _returnvalue (Utilities|Time|SetTimerbyEvent (delegate Custom|ChasingTraceTimer) 0.75 true))
  (bind _returnvalue_2 (Utilities|Time|SetTimerbyEvent (delegate Custom|Chasing) 0.5 true)))

(event Custom|StopChasing
  (Utilities|Time|ClearandInvalidateTimerbyHandle (stale Custom|BeginChase _returnvalue))
  (Utilities|Time|ClearandInvalidateTimerbyHandle (stale Custom|BeginChase _returnvalue_2)))