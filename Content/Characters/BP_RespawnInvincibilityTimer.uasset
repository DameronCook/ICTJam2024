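; BP_RespawnInvincibilityTimer grants temporary invincibility after respawn, with visual feedback on an optional mesh.
; BeginRespawnTimer sets IsInvincible, then runs a counted Delay loop in tenth-steps of InvincibilityTime before clearing it and restoring visibility.
; A FlipFlop blinks the static mesh, which takes priority; the skeletal mesh stays hidden throughout because its FlipFlop output is unconnected.
; With neither mesh valid, a single full-length Delay clears the flag.
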(event Custom|BeginRespawnTimer
  (Variables|Default|SetloopCounter 0)
  (Variables|Default|SetisInvincible true)
  (Variables|Default|GetstaticMeshToFlash
    (:then
      (bind _isa (Utilities|FlowControl|FlipFlop :!label _label)
        (:A
          _)
        (:B
          _))
      (Rendering|SetVisibility (Variables|Default|GetstaticMeshToFlash) (not _isa) false)
      (Math|Integer|IncrementInt (Variables|Default|GetloopCounter)
        (:%20%20
          (if (> (Variables|Default|GetloopCounter) 9)
            (Variables|Default|SetisInvincible false)
            (Rendering|SetVisibility (Variables|Default|GetstaticMeshToFlash) true false)
            (else
              (Utilities|FlowControl|Delay (/ (Variables|Default|GetinvincibilityTime) 1e+01))
              (goto _label))))))
    (:else
      (Variables|Default|GetskelMeshToFlash
        (:then
          (bind _isa_2 (Utilities|FlowControl|FlipFlop :!label _label_2)
            (:A
              _)
            (:B
              _))
          (Rendering|SetVisibility (Variables|Default|GetskelMeshToFlash) false false)
          (Math|Integer|IncrementInt (Variables|Default|GetloopCounter)
            (:%20%20
              (if (> (Variables|Default|GetloopCounter) 9)
                (Variables|Default|SetisInvincible false)
                (Rendering|SetVisibility (Variables|Default|GetskelMeshToFlash) true false)
                (else
                  (Utilities|FlowControl|Delay (/ (Variables|Default|GetinvincibilityTime) 1e+01))
                  (goto _label_2))))))
        (:else
          (Utilities|FlowControl|Delay (Variables|Default|GetinvincibilityTime))
          (Variables|Default|SetisInvincible false))))))