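; BP_Brute is an AI Brute whose overlap hitbox, labeled as a test, triggers the player's death.
; On overlap, it filters for actors implementing BPI_PlayerDeath whose respawn invincibility timer component reports not invincible.
; It then asks BP_ThirdPersonGameMode to change the player pawn using its DeathType, with a DoOnce reset after a short delay to throttle repeat triggers.
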(event EventBeginPlay
  (|CallParentFunction) ; This node is disabled and will not be called.\nDrag off pins to build functionality.
)

(event Collision|EventActorBeginOverlap
  (params (OtherActor :type Actor%20Object%20Reference))
  ;[0.5031 0.5031 0.5031] Test Hitbox
  (if (!= OtherActor self)
    (if (Utilities|DoesObjectImplementInterface OtherActor "/Game/_Core/BPI_PlayerDeath.BPI_PlayerDeath_C")
      (if (not (Variables|/Game/Characters/BP_RespawnInvincibilityTimer.BP_RespawnInvincibilityTimer_C|GetisInvincible (Actor|GetComponentbyClass OtherActor "/Game/Characters/BP_RespawnInvincibilityTimer.BP_RespawnInvincibilityTimer_C")))
        (Utilities|FlowControl|DoOnce false :!label _label
          (:Completed
            (Utilities|FlowControl|Sequence
              (:then_0
                (bind _asbp_third_person_game_mode (Utilities|Casting|CastToBP_ThirdPersonGameMode (Game|GetGameMode)))
                (Default|ChangePlayerPawn _asbp_third_person_game_mode (Variables|Default|GetdeathType))
                (Development|PrintString "Called change player spawn"))
              (:then_1
                (Utilities|FlowControl|Delay 3.0)
                (goto _label Reset)))))))))

(event EventTick
  (params (DeltaSeconds :type Float%20%28single-precision%29)))

(fn ConstructionScript
  (|CallParentFunction))